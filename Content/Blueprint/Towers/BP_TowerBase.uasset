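; BP_TowerBase is a tower Blueprint that fires homing projectiles when something enters its ShootRange.
; A begin overlap from anything not exactly of class BP_ProjectileTest starts a short delay, then spawns a BP_ProjectileTest at TowerTop facing ShootTarget.
; If ShootTarget is valid, the projectile homes on its scene component; ShootTarget is not assigned here, and the overlapping actor only serves the class check.
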(event OnComponentBeginOverlap(ShootRange)
  (params (OverlappedComponent :type Primitive%20Component%20Object%20Reference) (OtherActor :type Actor%20Object%20Reference) (OtherComp :type Primitive%20Component%20Object%20Reference) (OtherBodyIndex :type Integer) (bFromSweep :type Boolean) (SweepResult :type Hit%20Result%20Structure%20%28by%20ref%29))
  (bind _towertop (Variables|Default|GetTowerTop))
  (bind _shoottarget (Variables|Default|GetShootTarget))
  (bind _returnvalue (Transformation|GetWorldLocation _towertop))
  (if (not (== (Utilities|GetClass OtherActor) "/Game/Blueprint/Towers/BP_ProjectileTest.BP_ProjectileTest_C"))
    (Utilities|FlowControl|Delay 1.1)
    (bind _returnvalue_2 (Game|SpawnActorfromClass "/Game/Blueprint/Towers/BP_ProjectileTest.BP_ProjectileTest_C" (Math|Transform|MakeTransform _returnvalue (Math|Rotator|FindLookatRotation _returnvalue (Transformation|GetActorLocation (Variables|Default|GetShootTarget))) "1.000000,1.000000,1.000000") "AlwaysSpawn" 0 0))
    (Utilities|IsValid _shoottarget
      (:Is%20Valid
        (Variables|/Script/Engine.ProjectileMovementComponent|SetHomingTargetComponent (Variables|/Game/Blueprint/Towers/BP_ProjectileTest.BP_ProjectileTest_C|GetProjectileMovement _returnvalue_2) (Actor|GetComponentbyClass _shoottarget "/Script/Engine.SceneComponent"))
        (Variables|/Script/Engine.ProjectileMovementComponent|SetbIsHomingProjectile (Variables|/Game/Blueprint/Towers/BP_ProjectileTest.BP_ProjectileTest_C|GetProjectileMovement _returnvalue_2) true)))))

(fn ConstructionScript)