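; BP_TowerPlaceHolder is a clickable tower slot that offers a tower selection widget.
; On BeginPlay it hides its widget component, caches the WBP_SelectTowerToPlace instance and gives it a back-reference to itself.
; Clicking the static mesh prints a debug message and toggles the widget, unless that widget already holds a valid SpawnedTower.
; The TowerPlaced event hides the widget again.
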(event OnClicked(StaticMesh)
  (params (TouchedComponent :type Primitive%20Component%20Object%20Reference) (ButtonPressed :type Key%20Structure :default "None"))
  (Utilities|IsValid (Variables|/Game/Blueprint/Widgets/WBP_SelectTowerToPlace.WBP_SelectTowerToPlace_C|GetSpawnedTower (Variables|Default|GetAs%20WBP%20Select%20Tower%20To%20Place))
    (:Is%20Not%20Valid
      (Development|PrintString "PlaceHold has been touched" true true "(R=0.000000,G=1.000000,B=0.124176,A=1.000000)" 1e+01)
      (Rendering|ToggleVisibility (Variables|Default|GetWidget) false))))

(event Custom|TowerPlaced
  (Rendering|SetVisibility (Variables|Default|GetWidget) false false))

(event EventBeginPlay
  (Rendering|SetVisibility (Variables|Default|GetWidget) false false)
  (bind _aswbp_select_tower_to_place (Utilities|Casting|CastToWBP_SelectTowerToPlace (UserInterface|GetWidget (Variables|Default|GetWidget))))
  (bind _output_get (Variables|Default|SetAs%20WBP%20Select%20Tower%20To%20Place _aswbp_select_tower_to_place))
  (Variables|/Game/Blueprint/Widgets/WBP_SelectTowerToPlace.WBP_SelectTowerToPlace_C|SetOwningPlaceHolder _output_get self))

(fn ConstructionScript)