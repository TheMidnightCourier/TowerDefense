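; Player controller base that manages the visibility of widgets on tower placeholders in response to left mouse clicks.
; On BeginPlay it caches every BP_TowerPlaceHolder actor in the level.
; Each click traces under the cursor on the Visibility channel, hiding the widgets of all other placeholders when one is hit, or of every placeholder otherwise.
; It only hides widgets and never shows the clicked placeholder's own.
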(event EventBeginPlay
  (bind _outactors (Actor|GetAllActorsOfClass "/Game/Blueprint/Towers/BP_TowerPlaceHolder.BP_TowerPlaceHolder_C"))
  (Variables|Default|SetPlaceHolders _outactors))

(event EventTick
  (params (DeltaSeconds :type Float%20%28single-precision%29)))

(event Input|MouseEvents|LeftMouseButton
  (params (Key :type Key%20Structure :default "None"))
  (:Pressed
    (bind _asbp_tower_place_holder (Utilities|Casting|CastToBP_TowerPlaceHolder (.hitactor (.HitResult (Game|Player|GetHitResultUnderCursorbyChannel "TraceTypeQuery1" true))))
      (:then
        (for _array_element (Variables|Default|GetPlaceHolders)
          (if (not (== _array_element _asbp_tower_place_holder))
            (Rendering|SetVisibility (Variables|/Game/Blueprint/Towers/BP_TowerPlaceHolder.BP_TowerPlaceHolder_C|GetWidget _array_element) false false))))
      (:CastFailed
        (Utilities|FlowControl|Sequence
          (:then_0
            (for _array_element_2 (Variables|Default|GetPlaceHolders)
              (Rendering|SetVisibility (Variables|/Game/Blueprint/Towers/BP_TowerPlaceHolder.BP_TowerPlaceHolder_C|GetWidget _array_element_2) false false))))))))

(fn ConstructionScript)