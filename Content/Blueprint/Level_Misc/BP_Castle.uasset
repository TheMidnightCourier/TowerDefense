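; BP_Castle is the base the player defends, with a health pool that starts at DefaultHealth on BeginPlay.
; Its Box overlap destroys any overlapping BP_EnemyBase actor and decrements Health by one.
; At exactly zero it calls GameOver on BP_GameModeBase; otherwise it prints the remaining health on screen in red.
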(event OnComponentBeginOverlap(Box)
  (params (OverlappedComponent :type Primitive%20Component%20Object%20Reference) (OtherActor :type Actor%20Object%20Reference) (OtherComp :type Primitive%20Component%20Object%20Reference) (OtherBodyIndex :type Integer) (bFromSweep :type Boolean) (SweepResult :type Hit%20Result%20Structure%20%28by%20ref%29))
  (bind _asbp_enemy_base (Utilities|Casting|CastToBP_EnemyBase OtherActor))
  (Actor|DestroyActor _asbp_enemy_base)
  (bind _result (Math|Integer|DecrementInt (Variables|Default|GetHealth))
    (:%20%20
      (if (== _result 0)
        (bind _asbp_game_mode_base (Utilities|Casting|CastToBP_GameModeBase (Game|GetGameMode)))
        (Default|GameOver _asbp_game_mode_base)
        (else
          (Development|PrintString (Utilities|String|ToString(Integer) _result) true true "(R=0.729167,G=0.000000,B=0.037266,A=1.000000)" 1e+01))))))

(event EventBeginPlay
  (Variables|Default|SetHealth (Variables|Default|GetDefaultHealth)))

(event Collision|EventActorBeginOverlap
  (params (OtherActor :type Actor%20Object%20Reference)))

(event EventTick
  (params (DeltaSeconds :type Float%20%28single-precision%29)))

(fn ConstructionScript)