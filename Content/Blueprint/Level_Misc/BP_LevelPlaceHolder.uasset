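; BP_LevelPlaceHolder is a clickable level marker actor for the level choose map.
; On BeginPlay it builds a brush from its Image texture and parses the level number from a fixed two-character substring of LevelCodeName.
; Clicking its StaticMesh passes display name, code name, number and image to the LevelDescriptionWidget held by BP_GameMode_LevelChooseMap, then adds that widget to the viewport.
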(event OnClicked(StaticMesh)
  (params (TouchedComponent :type Primitive%20Component%20Object%20Reference) (ButtonPressed :type Key%20Structure :default "None"))
  (bind _asbp_game_mode_level_choose_map (Utilities|Casting|CastToBP_GameMode_LevelChooseMap (Game|GetGameMode)))
  (Default|SetupWidget (Variables|/Game/Blueprint/GameMode/BP_GameMode_LevelChooseMap.BP_GameMode_LevelChooseMap_C|GetLevelDescriptionWidget _asbp_game_mode_level_choose_map) (Variables|Description|GetLevelDisplayName) (Variables|Description|GetLevelCodeName) (Variables|Description|GetLevelNumber) (Variables|Description|GetLevelImage))
  (UserInterface|Viewport|AddtoViewport (Variables|/Game/Blueprint/GameMode/BP_GameMode_LevelChooseMap.BP_GameMode_LevelChooseMap_C|GetLevelDescriptionWidget _asbp_game_mode_level_choose_map) 0))

(event EventBeginPlay
  (Variables|Description|SetLevelImage (Class|WidgetBlueprintLibrary|MakeBrushfromTexture (Variables|Default|GetImage)))
  (Variables|Description|SetLevelNumber (Math|Conversions|ToInteger(Byte) (Utilities|String|GetSubstring (Utilities|String|ToString(Name) (Variables|Description|GetLevelCodeName)) 6 2))))

(event Collision|EventActorBeginOverlap
  (params (OtherActor :type Actor%20Object%20Reference)))

(event EventTick
  (params (DeltaSeconds :type Float%20%28single-precision%29)))

(fn ConstructionScript)