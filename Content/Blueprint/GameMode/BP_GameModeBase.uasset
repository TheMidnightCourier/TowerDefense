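; Game mode for a lane-based enemy wave game that spawns enemy groups, advances waves and shows gameplay and game-over widgets.
; A looping timer looks up request data table rows by composed level, wave, group and line names, with level parsed from the map name.
; SpawnGroup turns each row's enemy order into slow, base or fast enemies, offsets them in formation and starts them along their BP_TrackLine.
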(event Custom|DoRequest
  (bind _returnvalue (Class|DataTableFunctionLibrary|DoesDataTableRowExist (Variables|Default|GetDataSet) (Utilities|String|StringToName (Utilities|String|Append (Variables|Default|GetRequestName) (Utilities|String|ToString(Integer) (Variables|Default|GetCurrentLevel)) "W" (Utilities|String|ToString(Integer) (Variables|Default|GetCurrentWave)) "G" (Utilities|String|ToString(Integer) (Variables|Default|GetCurrentGroup)) "L" (Utilities|String|ToString(Integer) (Variables|Default|GetLine))))))
  (if _returnvalue
    (Utilities|FlowControl|ForLoopwithBreak 0 (Variables|Default|GetTrackLines) :!label _label
      (:LoopBody
        (bind _returnvalue_2 (Utilities|GetDataTableRow "/Game/Blueprint/GameMode/DT_Requests.DT_Requests" (Utilities|String|StringToName (Utilities|String|Append (Variables|Default|GetRequestName) (Utilities|String|ToString(Integer) (Variables|Default|GetCurrentLevel)) "W" (Utilities|String|ToString(Integer) (Variables|Default|GetCurrentWave)) "G" (Utilities|String|ToString(Integer) (Variables|Default|GetCurrentGroup)) "L" (Utilities|String|ToString(Integer) (Variables|Default|GetLine)))))
          (:then
            (Development|PrintString (Utilities|String|ToString(Name) (Utilities|String|StringToName (Utilities|String|Append (Variables|Default|GetRequestName) (Utilities|String|ToString(Integer) (Variables|Default|GetCurrentLevel)) "W" (Utilities|String|ToString(Integer) (Variables|Default|GetCurrentWave)) "G" (Utilities|String|ToString(Integer) (Variables|Default|GetCurrentGroup)) "L" (Utilities|String|ToString(Integer) (Variables|Default|GetLine))))) true true "(R=0.000000,G=0.660000,B=1.000000,A=1.000000)" 6e+01)
            (CallFunction|SpawnGroup (.Line (Utilities|Struct|BreakBP_SpawnRequest _returnvalue_2)) (.VerticalLines (Utilities|Struct|BreakBP_SpawnRequest _returnvalue_2)) (.HorizontalLines (Utilities|Struct|BreakBP_SpawnRequest _returnvalue_2)) (.EnemiesOrder (Utilities|Struct|BreakBP_SpawnRequest _returnvalue_2)))
            (Math|Integer|IncrementInt (Variables|Default|GetLine)))
          (:RowNotFound
            (goto _label Break))))
      (:Completed
        (Math|Integer|IncrementInt (Variables|Default|GetCurrentGroup)
          (:%20%20
            (Variables|Default|SetLine 1)))))))

(event Custom|WaveCleared
  (Math|Integer|IncrementInt (Variables|Default|GetCurrentWave)
    (:%20%20
      (Variables|Default|SetCurrentGroup 1)
      (Variables|Default|SetLine 1)
      (bind _returnvalue (Utilities|Time|SetTimerbyEvent (delegate Custom|DoRequest) 5.0 true -5.0))
      (Variables|Default|SetGroupSpawmTimer _returnvalue))))

(event Custom|GameOver
  (Development|PrintString "GameOver" true true "(R=0.729167,G=0.000000,B=0.037266,A=1.000000)" 1e+01)
  (Viewport|RemoveAllWidgets)
  (bind _returnvalue (UserInterface|CreateWidget "/Game/Blueprint/Widgets/WBP_GameOver.WBP_GameOver_C"))
  (UserInterface|Viewport|AddtoViewport _returnvalue 0))

(event EventBeginPlay
  (bind _returnvalue (Game|GetPlayerController 0))
  (bind _outactors (Actor|GetAllActorsOfClass "/Game/Blueprint/Level_Misc/BP_TrackLine.BP_TrackLine_C"))
  (Variables|Default|SetTrackLines (Utilities|Array|Length _outactors))
  (bind _returnvalue_2 (UserInterface|CreateWidget "/Game/Blueprint/Widgets/WBP_MainGamePlay.WBP_MainGamePlay_C"))
  (bind _output_get (Variables|Default|SetMainGameplayWidget _returnvalue_2))
  (UserInterface|Viewport|AddtoViewport _output_get 0)
  (Input|SetInputModeGameandUI _returnvalue 0 "DoNotLock" true)
  (Variables|/Script/Engine.PlayerController|SetbShowMouseCursor _returnvalue true)
  (bind _returnvalue_3 (Game|GetCurrentLevelName true))
  (Variables|Default|SetCurrentLevel (Math|Conversions|ToInteger(Byte) (Utilities|String|GetSubstring _returnvalue_3 6 2)))
  (bind _returnvalue_4 (Utilities|Time|SetTimerbyEvent (delegate Custom|DoRequest) 5.0 true -5.0))
  (Variables|Default|SetGroupSpawmTimer _returnvalue_4))

(fn ConstructionScript)

(fn SpawnGroup
  (params (Line :type Integer) (VerticalLines :type Integer) (HorizontalLines :type Integer) (EnemiesOrder :type Array%20of%20Integers))
  (bind _result (Math|Integer|DecrementInt Line)
    (:%20%20
      (LocalVariables|SetCurrentLine _result)
      (for (_array_element _array_index) EnemiesOrder
        (LocalVariables|SetVerticalLine (/ _array_index VerticalLines))
        (LocalVariables|SetHorizontalLine (Math|Integer|%(Integer) _array_index HorizontalLines))
        (LocalVariables|SetVerticalOffset (* (LocalVariables|GetVerticalOffsetPerLine) (LocalVariables|GetVerticalLine)))
        (LocalVariables|SetHorizontalOffset (* (LocalVariables|GetHorizontalOffsetPerLine) (LocalVariables|GetHorizontalLine)))
        (switch int _array_element
          (:1
            (bind _output_get (LocalVariables|SetSpawnClass "/Game/Blueprint/Enemies/BP_Enemy_Slow.BP_Enemy_Slow_C"))
            (bind _returnvalue (Game|SpawnActorfromClass _output_get (Math|Transform|MakeTransform "0, 0, 0" "0, 0, 0" "1.000000,1.000000,1.000000") "Undefined" 0 0))
            (LocalVariables|SetEnemy _returnvalue))
          (:2
            (bind _output_get_2 (LocalVariables|SetSpawnClass "/Game/Blueprint/Enemies/BP_EnemyBase.BP_EnemyBase_C"))
            (bind _returnvalue_2 (Game|SpawnActorfromClass _output_get_2 (Math|Transform|MakeTransform "0, 0, 0" "0, 0, 0" "1.000000,1.000000,1.000000") "Undefined" 0 0))
            (LocalVariables|SetEnemy _returnvalue_2))
          (:3
            (bind _output_get_3 (LocalVariables|SetSpawnClass "/Game/Blueprint/Enemies/BP_Enemy_Fast.BP_Enemy_Fast_C"))
            (bind _returnvalue_3 (Game|SpawnActorfromClass _output_get_3 (Math|Transform|MakeTransform "0, 0, 0" "0, 0, 0" "1.000000,1.000000,1.000000") "Undefined" 0 0))
            (LocalVariables|SetEnemy _returnvalue_3)))
        (bind _outactors (Actor|GetAllActorsOfClass "/Game/Blueprint/Level_Misc/BP_TrackLine.BP_TrackLine_C"))
        (Class|EnemyBase|SetTrackLine (LocalVariables|GetEnemy) (Utilities|Array|Get(acopy) _outactors (LocalVariables|GetCurrentLine)))
        (Class|EnemyBase|SetAlphaCurve (LocalVariables|GetEnemy) "/Game/Blueprint/Level_Misc/CF_CurveAlpha.CF_CurveAlpha")
        (Variables|/Script/TowerDefense.EnemyBase|SetVerticalOffset (LocalVariables|GetEnemy) (LocalVariables|GetVerticalOffset))
        (Transformation|AddRelativeLocation (Actor|GetComponentbyClass (LocalVariables|GetEnemy) "/Script/Engine.CapsuleComponent") (LocalVariables|GetHorizontalOffset) false false)
        (Class|EnemyBase|StartRunning (LocalVariables|GetEnemy))))))