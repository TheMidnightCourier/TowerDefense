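; BP_EnemyGroup lays out a grid of scene components, apparently as position slots for a group of enemies, and spawns no enemies itself.
; Its construction script loops over VerticalLines and HorizontalLines, stepping rows along negative Y and offsetting columns along X.
; Only the first three column indices add components, and the middle one reuses the previous X offset instead of setting its own.
; Each new component's name is printed; BeginPlay is empty.
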(event EventBeginPlay)

(fn ConstructionScript
  (for _index (range 0 (Variables|Default|GetVerticalLines))
    (Variables|Default|SetVerticalOffset (Math|Vector|MakeVector 0.0 (Math|Conversions|ToFloat(Integer) (* _index -100)) 0.0))
    (for _index_2 (range 0 (Variables|Default|GetHorizontalLines))
      (switch int _index_2
        (:0
          (Variables|Default|SetHorizontalOffset "-100.000000, 0, 0"))
        (:1
          _)
        (:2
          (Variables|Default|SetHorizontalOffset "100.000000, 0, 0")))
      (bind _output_get (Variables|Default|SetOffset (+ (Variables|Default|GetVerticalOffset) (Variables|Default|GetHorizontalOffset))))
      (bind _returnvalue (AddComponent|AddSceneComponent false (Math|Transform|MakeTransform _output_get "0, 0, 0" "1.000000,1.000000,1.000000")))
      (Development|PrintString (Utilities|GetObjectName _returnvalue)))))